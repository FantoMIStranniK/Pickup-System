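; BP_Item is a world pickup actor for the pickup system, representing one item identified by a DataTable and row name.
; SetData stores that table and row on the actor, and BeginPlay caches the game state cast to GS_PickupSystem.
; PickUp passes the table and row to the game state's AddItem, then destroys the actor.
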(event EventBeginPlay
  (bind _asgs_pickup_system (Utilities|Casting|CastToGS_PickupSystem (Game|GetGameState)))
  (Variables|Default|SetGameState _asgs_pickup_system))

(fn ConstructionScript)

(fn PickUp
  (Default|AddItem (Variables|Default|GetGameState) (Variables|Default|GetDataTable) (Variables|Default|GetItemName))
  (Actor|DestroyActor))

(fn SetData
  (params (DataTable :type Data%20Table%20Object%20Reference) (RowName :type Name))
  (Variables|Default|SetDataTable DataTable)
  (Variables|Default|SetItemName RowName))